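; Zombie enemy that wanders randomly, hunts the player on sight, sound or non-head damage, and attacks in melee.
; AIMoveTo loops drive patrol and chase, while Tick handles death, target loss by distance or player death, and focus.
; Random left or right montages set damage, which hand overlaps apply while the Attack flag is on.
; Headshots kill instantly, hits show a hitmarker, and death ragdolls only near stairs.
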(event `self.ReceiveTick`
  (params (DeltaSeconds :type "Float (single-precision)"))
  (if (<= (`self.CurrentHealth`) 0.0)
    ;[1 1 1] Zombie dies
    (set `self.IsDead?` true)
    (`MovementComponent.StopMovementImmediately` (`self.CharacterMovement`))
    (`PrimitiveComponent.SetCollisionEnabled` (`self.CapsuleComponent`) "NoCollision")
    (`AIController.K2_SetFocus` (cast `AIController` (`self.GetController`) :!pure true) null)
    (if (`self.IsStairsNearby?`)
      (`KismetSystemLibrary.Delay` 2.5)
      (`SkeletalMeshComponent.SetAllBodiesSimulatePhysics` (`self.Mesh`) true)
      (`PrimitiveComponent.SetCollisionEnabled` (`self.Mesh`) "QueryAndPhysics"))
    (elif (`/Game/ThirdPersonBP/Blueprints/Character/BP_ThirdPersonCharacter.IsDead?` (cast `/Game/ThirdPersonBP/Blueprints/Character/BP_ThirdPersonCharacter` (`GameplayStatics.GetPlayerCharacter` 0) :!pure true))
      ;[1 1 1] If charachter dead
      (`/Engine/EditorBlueprintResources/StandardMacros.DoOnce` false
        (:`Completed`
          (`self.ResetPawnSensing`)
          (set `self.EnemyFound?` false)
          (set `CharacterMovementComponent.MaxWalkSpeed` 100.0 (`self.CharacterMovement`))
          (`MovementComponent.StopMovementImmediately` (`self.CharacterMovement`))
          (`KismetSystemLibrary.Delay` (`KismetMathLibrary.RandomFloatInRange` 3.0 6.0))
          (`AIController.K2_SetFocus` (cast `AIController` (`self.GetController`) :!pure true) null)
          (`self.AIMovement`)))
      (elif (not (`self.IsDead?`))
        (`|ExecutionSequence`
          (:`then_0`
            ;[1 1 1] Condition for hunting player
            (if (`self.EnemyFound?`)
              (`/Engine/EditorBlueprintResources/StandardMacros.DoOnce` false :!label _label
                (:`Completed`
                  (`AIController.K2_SetFocus` (cast `AIController` (`self.GetController`) :!pure true) (cast `/Game/ThirdPersonBP/Blueprints/Character/BP_ThirdPersonCharacter` (`GameplayStatics.GetPlayerCharacter` 0) :!pure true))
                  (`self.HuntPlayer`)))
              (else
                (goto _label :!via `Reset`))))
          (:`then_1`
            ;[1 1 1] Zombie losses charchter
            (if (>= (`self.GetDistanceTo` (cast `/Game/ThirdPersonBP/Blueprints/Character/BP_ThirdPersonCharacter` (`GameplayStatics.GetPlayerCharacter` 0) :!pure true)) 1000.0)
              (`/Engine/EditorBlueprintResources/StandardMacros.DoOnce` false :!label _label_2
                (:`Completed`
                  (set `self.EnemyFound?` false)
                  (`self.ResetPawnSensing`)
                  (`MovementComponent.StopMovementImmediately` (`self.CharacterMovement`))
                  (set `CharacterMovementComponent.MaxWalkSpeed` 100.0 (`self.CharacterMovement`))
                  (`AIController.K2_SetFocus` (cast `AIController` (`self.GetController`) :!pure true) null)
                  (`KismetSystemLibrary.Delay` (`KismetMathLibrary.RandomFloatInRange` 3.0 6.0))
                  (`self.AIMovement`)))
              (else
                (goto _label_2 :!via `Reset`)))))))))

(event `self.ReceiveBeginPlay`
  ;[1 1 1] Begin play
  (set `self.CurrentHealth` (`self.MaxHealth`))
  (`self.AIMovement`))

(event `AIMovement`
  ;[1 1 1] Zombie patrols the area
  (if (`self.IsDead?`)
    _
    (elif (not (`self.EnemyFound?`))
      (`|AIMoveTo` self (`NavigationSystem.K2_GetRandomReachablePointInRadius` (`self.K2_GetActorLocation`) 700.0 null "/Script/AIModule.NavFilter_AIControllerDefault")
        (:`OnSuccess`
          (`KismetSystemLibrary.Delay` (`KismetMathLibrary.RandomFloatInRange` 2.0 6.0) :!label _label_3)
          (`self.AIMovement`))
        (:`OnFail`
          (if (`self.IsDead?`)
            _
            (elif (not (`self.EnemyFound?`))
              (goto _label_3))))))))

(event `HuntPlayer`
  ;[1 1 1] Hunt player
  (if (`self.IsDead?`)
    _
    (elif (`self.EnemyFound?`)
      (set `CharacterMovementComponent.MaxWalkSpeed` 300.0 (`self.CharacterMovement`))
      (`|AIMoveTo` self (0.0 0.0 0.0) (`GameplayStatics.GetPlayerCharacter` 0) 50.0 true
        (:`OnSuccess`
          (`self.AttackPlayer`))
        (:`OnFail`
          (if (`self.EnemyFound?`)
            (`KismetSystemLibrary.Delay` 0.2)
            (`self.HuntPlayer`)))))))

(event `/Game/AI/ZombieBP/DamageBP/TakeDamage.ITakeDamage`
  (params (BoneName :type Name) (Damage :type "Float (single-precision)"))
  ;[1 1 1] Zombie takes damage
  (`|ExecutionSequence`
    (:`then_0`
      (if (== BoneName "head")
        (set `self.CurrentHealth` 0.0)
        (`KismetSystemLibrary.PrintString` "Headshot!")
        (else
          (set `self.CurrentHealth` (- (`self.CurrentHealth`) Damage))
          (set `self.EnemyFound?` true))))
    (:`then_1`
      (bind _returnvalue (`|CreateWidget` "/Game/ThirdPersonBP/UI/Hitmarker.Hitmarker_C"))
      (`UserWidget.AddToViewport` _returnvalue 0)
      (`KismetSystemLibrary.Delay` 1.0)
      (`Widget.RemoveFromParent` _returnvalue))))

(event `AttackPlayer`
  ;[1 1 1] Attack anim logic
  (switch `int` (`KismetMathLibrary.RandomIntegerInRange` 0 1)
    (:`0`
      (set `self.ZombieDamage` 10.0)
      (`self.PlayAnimMontage` "/Game/AI/ZombieBP/ZombieAnimation/Zombie_Right_Attack_Anim_Montage.Zombie_Right_Attack_Anim_Montage" 1.5)
      (`KismetSystemLibrary.Delay` 1.5))
    (:`1`
      (set `self.ZombieDamage` 15.0)
      (`self.PlayAnimMontage` "/Game/AI/ZombieBP/ZombieAnimation/Zombie_Left_Attack_Anim_Montage.Zombie_Left_Attack_Anim_Montage" 1.5)
      (`KismetSystemLibrary.Delay` 1.5)))
  (`self.HuntPlayer`))

(event `OnAttack`
  (set `self.Attack` true))

(event `OffAttack`
  (set `self.Attack` false))

(event `self.PawnSensing.OnSeePawn`
  (params (Pawn :type "Pawn Object Reference"))
  ;[1 1 1] Zombie sees charachter
  (if (not (`self.IsDead?`))
    (bind _asbp_third_person_character (cast `/Game/ThirdPersonBP/Blueprints/Character/BP_ThirdPersonCharacter` Pawn))
    (if (not (`/Game/ThirdPersonBP/Blueprints/Character/BP_ThirdPersonCharacter.IsDead?` _asbp_third_person_character))
      (`/Engine/EditorBlueprintResources/StandardMacros.DoOnce` false :!label _label_4
        (:`Completed`
          (set `self.EnemyFound?` true))))))

(event `self.RightHand.OnComponentBeginOverlap`
  (params (OverlappedComponent :type "PrimitiveComponent Object Reference") (OtherActor :type "Actor Object Reference") (OtherComp :type "PrimitiveComponent Object Reference") (OtherBodyIndex :type Integer) (bFromSweep :type Boolean) (SweepResult :type "HitResult Structure (by ref)"))
  ;[1 1 1] Zombie hit player with right and left hand
  (if (`self.Attack`)
    (bind _asbp_third_person_character (cast `/Game/ThirdPersonBP/Blueprints/Character/BP_ThirdPersonCharacter` OtherActor))
    (`/Game/ThirdPersonBP/Blueprints/Character/BP_ThirdPersonCharacter.Event ITake Damage` _asbp_third_person_character "None" (`self.ZombieDamage`))))

(event `ResetPawnSensing`
  ;[1 1 1] Zombie sees charachter
  (goto _label_4 :!via `Reset`))

(event `self.LeftHand.OnComponentBeginOverlap`
  (params (OverlappedComponent :type "PrimitiveComponent Object Reference") (OtherActor :type "Actor Object Reference") (OtherComp :type "PrimitiveComponent Object Reference") (OtherBodyIndex :type Integer) (bFromSweep :type Boolean) (SweepResult :type "HitResult Structure (by ref)"))
  ;[1 1 1] Zombie hit player with right and left hand
  (if (`self.Attack`)
    (bind _asbp_third_person_character (cast `/Game/ThirdPersonBP/Blueprints/Character/BP_ThirdPersonCharacter` OtherActor))
    (`/Game/ThirdPersonBP/Blueprints/Character/BP_ThirdPersonCharacter.Event ITake Damage` _asbp_third_person_character "None" (`self.ZombieDamage`))))

(event `self.PawnSensing.OnHearNoise`
  (params (Instigator :type "Pawn Object Reference") (Location :type "Vector Structure (by ref)") (Volume :type "Float (single-precision)"))
  (if (not (`self.IsDead?`))
    (`KismetSystemLibrary.PrintString` "Zombie: I hear you!!!!")
    (set `self.EnemyFound?` true)
    (`self.HuntPlayer`)))

(fn `UserConstructionScript`)